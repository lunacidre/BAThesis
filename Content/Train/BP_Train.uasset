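; Train actor that travels along the spline of a referenced track when flagged active at BeginPlay.
; A timeline, with play rate set from Duration and start time from an offset, drives an alpha from which each update derives a distance along the spline.
; The actor takes the world-space location and rotation at that distance, so it follows the track's path and orientation.
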(event `self.ReceiveBeginPlay`
  (if (`self.ActiveTrain`)
    (`self.MoveTrain`)))

(event `MoveTrain`
  (bind _returnvalue (`KismetMathLibrary.Lerp` 0.0 (`SplineComponent.GetSplineLength` (`/Game/Train/BP_TrainTrack.UsefulSpline` (`self.TrackRef`))) (`self.Alpha`)))
  (`TimelineComponent.SetPlayRate` (`self.TrainMover`) (/ 1.0 (`self.Duration`)))
  (`TimelineComponent.SetNewTime` (`self.TrainMover`) (`self.TrainStrartOffset`))
  (bind (_direction _alpha) (`Timeline|TrainMover`)
    (:`Update`
      (set `self.Alpha` _alpha)
      (`self.K2_SetActorLocationAndRotation` (`SplineComponent.GetLocationAtDistanceAlongSpline` (`/Game/Train/BP_TrainTrack.UsefulSpline` (`self.TrackRef`)) _returnvalue "World") (`SplineComponent.GetRotationAtDistanceAlongSpline` (`/Game/Train/BP_TrainTrack.UsefulSpline` (`self.TrackRef`)) _returnvalue "World")))))

(fn `UserConstructionScript`)